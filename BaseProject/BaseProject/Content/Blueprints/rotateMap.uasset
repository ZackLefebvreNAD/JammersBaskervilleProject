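; rotateMap is a Blueprint that spins its Cube component around the Z axis from horizontal mouse movement.
; The MouseX axis event applies a very large physics torque scaled by axis value and Tick's delta time.
; BeginPlay prints the player pawn's name and Tick prints the torque vector, apparently for debugging.
; An EnableInput node for the player controller is present but unconnected, so it never runs.
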(event `self.ReceiveBeginPlay`
  (`KismetSystemLibrary.PrintString` (`KismetSystemLibrary.GetDisplayName` (`GameplayStatics.GetPlayerPawn` 0))))

(event `InputAxisKey|MouseX`
  (params (AxisValue :type "Float (single-precision)"))
  (`PrimitiveComponent.AddTorqueInRadians` (`self.Cube`) (`KismetMathLibrary.MakeVector` 0.0 0.0 (* AxisValue 30000000000.0 (stale `self.ReceiveTick` DeltaSeconds))) "None" false))

(event `self.ReceiveTick`
  (params (DeltaSeconds :type "Float (single-precision)"))
  (`KismetSystemLibrary.PrintString` (`KismetStringLibrary.Conv_VectorToString` (`KismetMathLibrary.MakeVector` 0.0 0.0 (* (stale `InputAxisKey|MouseX` AxisValue) 30000000000.0 DeltaSeconds)))))

(fn `UserConstructionScript`)