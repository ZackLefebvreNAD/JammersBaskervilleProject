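; Player character with jumping, interaction, key pickup and door teleportation.
; F scans overlapped interaction blocks to collect keys or toggle switches that set door states by DoorID, then teleports through overlapped doors after a camera fade if any key is held, without consuming it.
; Movement input is added once per movable object in the level, slowed for those overlapping the Box.
; Tick locks actor rotation to zero.
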(event `Key|F`
  (params (Key :type "Key Structure"))
  (:`Pressed`
    (`|ExecutionSequence`
      (:`then_0`
        (`KismetSystemLibrary.PrintString` "Using")
        (bind _outactors (`GameplayStatics.GetAllActorsOfClass` "/Game/MyContent/LevelBlockBPs/BP_InteractionBlock.BP_InteractionBlock_C"))
        (for _array_element _outactors
          (if (`self.IsOverlappingActor` _array_element)
            (if (`/Game/MyContent/LevelBlockBPs/BP_InteractionBlock.isKey?` _array_element)
              (`/Engine/EditorBlueprintResources/StandardMacros.IncrementInt` (`self.keys`)
                (:`  `
                  (`KismetSystemLibrary.PrintString` "Took a key")
                  (`self.K2_DestroyActor` _array_element)))
              (else
                (bind _output_get (set `/Game/MyContent/LevelBlockBPs/BP_InteractionBlock.isEnabled?` (not (`/Game/MyContent/LevelBlockBPs/BP_InteractionBlock.isEnabled?` _array_element)) _array_element))
                (if _output_get
                  (bind _outactors_2 (`GameplayStatics.GetAllActorsOfClass` "/Game/MyContent/LevelBlockBPs/BP_TeleportationDoor.BP_TeleportationDoor_C"))
                  (for _array_element_2 _outactors_2
                    (set `/Game/MyContent/LevelBlockBPs/BP_TeleportationDoor.Enabled?` (== (`/Game/MyContent/LevelBlockBPs/BP_TeleportationDoor.doorID` _array_element_2) (`/Game/MyContent/LevelBlockBPs/BP_InteractionBlock.doorID` _array_element)) _array_element_2))))))))
      (:`then_1`
        (bind _outactors_3 (`GameplayStatics.GetAllActorsOfClass` "/Game/MyContent/LevelBlockBPs/BP_TeleportationDoor.BP_TeleportationDoor_C"))
        (for _array_element_3 _outactors_3
          (if (`self.IsOverlappingActor` _array_element_3)
            (if (>= (`self.keys`) 1)
              (set `/Game/MyContent/LevelBlockBPs/BP_TeleportationDoor.Enabled?` true _array_element_3)
              (`PlayerCameraManager.StartCameraFade` :`self` (`GameplayStatics.GetPlayerCameraManager` 0) :`ToAlpha` 1.0 :`Duration` 1.0)
              (`KismetSystemLibrary.Delay` 1.0)
              (`self.K2_SetActorLocation` (`/Game/MyContent/LevelBlockBPs/BP_TeleportationDoor.New Location` _array_element_3) false true))))))))

(event `Key|SpaceBar`
  (params (Key :type "Key Structure"))
  (:`Pressed`
    (`KismetSystemLibrary.PrintString` "Jump")
    (`self.Jump`)))

(event `InputAxis|Move Forward`
  (params (AxisValue :type "Float (single-precision)"))
  (bind _returnvalue (`SceneComponent.GetForwardVector` (`self.CapsuleComponent`)))
  (bind _outactors (`GameplayStatics.GetAllActorsOfClass` "/Game/MyContent/Blueprints/movableObjectTemplate_Blueprint.movableObjectTemplate_Blueprint_C"))
  (for _array_element _outactors
    (if (`PrimitiveComponent.IsOverlappingActor` (`self.Box`) _array_element)
      (`self.AddMovementInput` _returnvalue (* (`self.SlowWhenCollision`) AxisValue))
      (else
        (`self.AddMovementInput` _returnvalue AxisValue)))))

(event `InputAxis|Move Right`
  (params (AxisValue :type "Float (single-precision)"))
  (bind _returnvalue (`SceneComponent.GetRightVector` (`self.CapsuleComponent`)))
  (bind _outactors (`GameplayStatics.GetAllActorsOfClass` "/Game/MyContent/Blueprints/movableObjectTemplate_Blueprint.movableObjectTemplate_Blueprint_C"))
  (for _array_element _outactors
    (if (`PrimitiveComponent.IsOverlappingActor` (`self.Box`) _array_element)
      (`self.AddMovementInput` _returnvalue (* AxisValue (`self.SlowWhenCollision`)))
      (else
        (`self.AddMovementInput` _returnvalue AxisValue)))))

(event `self.ReceiveTick`
  (params (DeltaSeconds :type "Float (single-precision)"))
  (`self.K2_SetActorRotation` (struct)))

(fn `UserConstructionScript`)