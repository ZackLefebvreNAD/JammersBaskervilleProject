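; BP_Player is a player character Blueprint with basic movement, jump and a placeholder use action.
; Move Forward and Move Right axis inputs add movement along the capsule component's forward and right vectors.
; Space Bar and F are bound directly as key events: Space Bar prints a debug string and jumps, while F only prints "Using".
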(event `Key|F`
  (params (Key :type "Key Structure"))
  (:`Pressed`
    (`KismetSystemLibrary.PrintString` "Using")))

(event `Key|SpaceBar`
  (params (Key :type "Key Structure"))
  (:`Pressed`
    (`KismetSystemLibrary.PrintString` "Jump")
    (`self.Jump`)))

(event `InputAxis|Move Forward`
  (params (AxisValue :type "Float (single-precision)"))
  (`self.AddMovementInput` (`SceneComponent.GetForwardVector` (`self.CapsuleComponent`)) AxisValue))

(event `InputAxis|Move Right`
  (params (AxisValue :type "Float (single-precision)"))
  (`self.AddMovementInput` (`SceneComponent.GetRightVector` (`self.CapsuleComponent`)) AxisValue))

(fn `UserConstructionScript`)