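; Floor actor that lets the player turn it with the mouse and push named static mesh blocks around by dragging.
; Holding the right button yaws the root by MouseX input.
; The moveblock3 event finds the named StaticMeshActor and records the cursor start position.
; Until left-button release, Tick searches all StaticMeshActors by display name and applies horizontal force to the match, scaled from the cursor's offset since the grab.
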(event `InputAxisKey|MouseX`
  (params (AxisValue :type "Float (single-precision)")))

(event `InputAxisKey|MouseX`
  (params (AxisValue :type "Float (single-precision)"))
  (if (`self.rihgtmouse`)
    (`SceneComponent.K2_AddWorldRotation` (`self.DefaultSceneRoot`) (`KismetMathLibrary.MakeRotator` 0.0 0.0 AxisValue) false false)))

(event `self.ReceiveTick`
  (params (DeltaSeconds :type "Float (single-precision)"))
  (bind _outactors (`GameplayStatics.GetAllActorsOfClass` "/Script/Engine.StaticMeshActor"))
  (for _array_element _outactors
    (if (`KismetStringLibrary.EqualEqual_StrStr` (`KismetSystemLibrary.GetDisplayName` _array_element) (stale `moveblock3` name))
      (if (`self.IsClicked`)
        (bind _returnvalue (`WidgetLayoutLibrary.GetMousePositionOnViewport`))
        (bind (_returnvalue_x _returnvalue_y _returnvalue_z) (`KismetMathLibrary.BreakVector` (* (+ (- (`self.initMousePos`) _returnvalue) (0.0 0.0 0.0)) (-20.0 20.0 0.0) 6)))
        (`PrimitiveComponent.AddForce` (`StaticMeshActor.StaticMeshComponent` _array_element) (`KismetMathLibrary.MakeVector` _returnvalue_y _returnvalue_x _returnvalue_z) "None" false)))))

(event `moveblock3`
  (params (name :type String))
  (bind _outactors (`GameplayStatics.GetAllActorsOfClass` "/Script/Engine.StaticMeshActor"))
  (for _array_element _outactors
    (bind _returnvalue (`KismetSystemLibrary.GetDisplayName` _array_element))
    (if (`KismetStringLibrary.EqualEqual_StrStr` _returnvalue name)
      (`KismetSystemLibrary.PrintString` _returnvalue)
      (bind _returnvalue_2 (`WidgetLayoutLibrary.GetMousePositionOnViewport`))
      (set `self.initMousePos` (`KismetMathLibrary.Conv_Vector2DToVector` _returnvalue_2))
      (set `self.initCharacter` (`self.K2_GetActorLocation` _array_element))
      (set `self.IsClicked` true))))

(event `Key|LeftMouseButton`
  (params (Key :type "Key Structure"))
  (:`Released`
    (set `self.IsClicked` false)))

(event `Key|RightMouseButton`
  (params (Key :type "Key Structure"))
  (:`Pressed`
    (set `self.rihgtmouse` true))
  (:`Released`
    (set `self.rihgtmouse` false)))

(fn `UserConstructionScript`)