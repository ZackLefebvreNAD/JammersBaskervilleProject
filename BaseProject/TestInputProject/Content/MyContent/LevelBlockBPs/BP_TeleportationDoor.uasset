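; Level-block door that teleports whatever actor overlaps its collision to a set location.
; While enabled and not already active, an overlap fades the player camera out and shows Arm and Keys widgets in a staggered sequence before moving the actor.
; An Active flag blocks re-triggering until the teleport completes.
; The construction script applies the configurable door mesh.
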(event `self.DoorCollision.OnComponentBeginOverlap`
  (params (OverlappedComponent :type "PrimitiveComponent Object Reference") (OtherActor :type "Actor Object Reference") (OtherComp :type "PrimitiveComponent Object Reference") (OtherBodyIndex :type Integer) (bFromSweep :type Boolean) (SweepResult :type "HitResult Structure (by ref)"))
  (if (`self.Enabled?`)
    (if (not (`self.active`))
      (set `self.active` true)
      (`PlayerCameraManager.StartCameraFade` :`self` (`GameplayStatics.GetPlayerCameraManager` 0) :`ToAlpha` 1.0 :`Duration` 1.0)
      (bind _returnvalue (`|CreateWidget` "/Game/MyContent/Widgets/Arm.Arm_C"))
      (`UserWidget.AddToViewport` _returnvalue 0)
      (`KismetSystemLibrary.Delay` 0.3)
      (bind _returnvalue_2 (`|CreateWidget` "/Game/MyContent/Widgets/Keys.Keys_C"))
      (`UserWidget.AddToViewport` _returnvalue_2 0)
      (`KismetSystemLibrary.Delay` 1.0)
      (`self.K2_SetActorLocation` OtherActor (`self.New Location`) false true)
      (set `self.active` false))))

(fn `UserConstructionScript`
  (`StaticMeshComponent.SetStaticMesh` (`self.Door`) (`self.Door Mesh`)))